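; Board Blueprint that builds a checkerboard of static mesh tiles, sized by SizeX and SizeY.
; The construction script runs nested loops, adding one mesh component per cell at AssetSize spacing, starting one cell away from the origin.
; The parity of row plus column selects oak or pine wood material for each tile.
; The event graph holds only disabled default events.
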(fn `UserConstructionScript`
  (bind _assetsize (`self.AssetSize`))
  (for _index (range 1 (+ (`self.SizeY`) 1))
    (for _index_2 (range 1 (+ (`self.SizeX`) 1))
      (bind _returnvalue (`AddComponent|NODE_AddStaticMeshComponent-0` :`RelativeTransform` (`KismetMathLibrary.MakeTransform` (`KismetMathLibrary.MakeVector` (`KismetMathLibrary.Conv_IntToDouble` (* _assetsize _index_2)) (`KismetMathLibrary.Conv_IntToDouble` (* _index _assetsize))))))
      (`PrimitiveComponent.SetMaterial` _returnvalue 0 (select `int` (mod (+ _index _index_2) 2) :`0` "/Game/StarterContent/Materials/M_Wood_Oak.M_Wood_Oak" :`1` "/Game/StarterContent/Materials/M_Wood_Pine.M_Wood_Pine" :!type "MaterialInterface Object Reference")))))